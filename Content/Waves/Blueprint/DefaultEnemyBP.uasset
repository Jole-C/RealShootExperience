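; Default enemy for the waves game, which homes in on the player and self-destructs on contact.
; After a zero-length delay at BeginPlay, its ProjectileMovement targets the CharacterReference root component for homing.
; A player pawn entering PlayerDetectionRadius takes damage and the enemy destroys itself without awarding score.
; DamageEnemy reduces health and, once it is depleted, destroys the actor, then calls ApplyComboAndScore.
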(event Custom|OnComponentBeginOverlap_Event
  (params (OverlappedComponent :type Primitive%20Component%20Object%20Reference) (OtherActor :type Actor%20Object%20Reference) (OtherComp :type Primitive%20Component%20Object%20Reference) (OtherBodyIndex :type Integer) (bFromSweep :type Boolean) (SweepResult :type Hit%20Result%20Structure%20%28by%20ref%29))
  (if (== OtherActor (Game|Player|GetPlayerPawn 0))
    (bind _asbp_first_person_character (Utilities|Casting|CastToBP_FirstPersonCharacter OtherActor))
    (Game|Damage|ApplyDamage _asbp_first_person_character 1.0 0 0)
    (Actor|DestroyActor)))

(event EventBeginPlay
  (|CallParentFunction)
  (Utilities|FlowControl|Sequence
    (:then_0
      (Utilities|FlowControl|Delay 0.0)
      (Variables|/Script/Engine.ProjectileMovementComponent|SetHomingTargetComponent (Variables|Default|GetProjectileMovement) (Variables|/Script/Engine.Actor|GetRootComponent (Variables|Default|GetCharacterReference))))
    (:then_1
      (Collision|AssignOnComponentBeginOverlap (Variables|Default|GetPlayerDetectionRadius) (delegate Custom|OnComponentBeginOverlap_Event)))))

(event EventEndPlay
  (params (EndPlayReason :type EEndPlayReason%20Enum :default "Destroyed"))
  (|CallParentFunction EndPlayReason))

(event EventDamageEnemy
  (params (damageAmount :type Integer))
  (bind _output_get (Variables|Default|SetEnemyHealth (- (Variables|Default|GetEnemyHealth) damageAmount)))
  (if (<= _output_get 0)
    (Actor|DestroyActor)
    (Class|EnemyBase|ApplyComboandScore)))

(fn ConstructionScript)