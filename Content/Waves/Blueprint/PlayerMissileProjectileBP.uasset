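; PlayerMissileProjectileBP is the player's missile, which damages weakpoints or breaks the score combo.
; Each overlap on its PlayerBullet-profile collision records whether the touched component is attached to a WeakpointBase.
; Hit logic runs on EndPlay: a flagged hit sphere-traces for nearby weakpoints and calls OnWeakpointHit on them, otherwise the ScoreManager combo resets.
; EndPlay also spawns the explosion effect at the missile's location.
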(event Custom|OnOverlap
  (params (OverlappedComponent :type Primitive%20Component%20Object%20Reference) (OtherActor :type Actor%20Object%20Reference) (OtherComp :type Primitive%20Component%20Object%20Reference) (OtherBodyIndex :type Integer) (bFromSweep :type Boolean) (SweepResult :type Hit%20Result%20Structure%20%28by%20ref%29))
  (Utilities|Casting|CastToWeakpointBase (Transformation|GetAttachParent OtherComp)
    (:then
      (Variables|Default|SetDidHitWeakpoint true)
      (Development|PrintString "Hit Weakpoint"))
    (:CastFailed
      (Variables|Default|SetDidHitWeakpoint false))))

(event EventBeginPlay
  (Utilities|FlowControl|Sequence
    (:then_0
      (Collision|AssignOnComponentBeginOverlap (Variables|Default|GetCollisionComp) (delegate Custom|OnOverlap)))
    (:then_1
      (bind _returnvalue (Actor|GetActorOfClass "/Game/Waves/Blueprint/ScoreManagerBP.ScoreManagerBP_C"))
      (Variables|Default|SetScoreManagerReference _returnvalue)
      (Collision|SetCollisionProfileName (Variables|Default|GetCollisionComp) "PlayerBullet" true :!class /Script/Engine.PrimitiveComponent))))

(event EventEndPlay
  (params (EndPlayReason :type EEndPlayReason%20Enum :default "Destroyed"))
  (bind _returnvalue (Transformation|GetActorLocation))
  (Utilities|FlowControl|Sequence
    (:then_0
      (if (Variables|Default|GetDidHitWeakpoint)
        (bind _outhits (Collision|MultiSphereTraceByChannel _returnvalue _returnvalue 1.5e+02 "TraceTypeQuery3" false 0 "None"))
        (bind _output_get (Variables|Default|SetOut%20Hits _outhits))
        (for _array_element _output_get
          (bind _asweakpoint_base (Utilities|Casting|CastToWeakpointBase (Transformation|GetAttachParent (.HitComponent (Collision|BreakHitResult _array_element)))))
          (Class|WeakpointBase|OnWeakpointHit _asweakpoint_base)
          (Development|PrintString "Hit weakpoint.")
          (Actor|DestroyActor))
        (else
          (Class|ScoreManager|ResetCombo (Variables|Default|GetScoreManagerReference))
          (Development|PrintString "Did not hit Weakpoint"))))
    (:then_1
      (Niagara|SpawnSystematLocation "/Game/Waves/Niagara/PlayerMissileExplosion.PlayerMissileExplosion" (Transformation|GetActorLocation)))))

(fn ConstructionScript
  (|CallParentFunction))