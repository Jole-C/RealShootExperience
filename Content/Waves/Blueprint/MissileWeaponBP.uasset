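; MissileWeaponBP is a player weapon that fires missile projectiles.
; When CanFire is true, Fire spawns a triple-scale PlayerMissileProjectileBP at the muzzle, oriented by the player camera's rotation rather than the weapon's.
; It then shakes the camera, calls HandleClip and plays an attenuated firing sound at the actor's location.
; The Fire event's line trace comment does not match the graph, which performs no trace.
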(event EventBeginPlay)

(event Collision|EventActorBeginOverlap
  (params (OtherActor :type Actor%20Object%20Reference)))

(event EventTick
  (params (DeltaSeconds :type Float%20%28single-precision%29)))

(event EventFire
  ;[1 1 1] Generate line trace on hit
  (if (Variables|Default|GetCanFire)
    (Utilities|FlowControl|Sequence
      (:then_0
        (Game|SpawnActorfromClass "/Game/Waves/Blueprint/PlayerMissileProjectileBP.PlayerMissileProjectileBP_C" (Math|Transform|MakeTransform (Transformation|GetWorldLocation (Variables|Default|GetMuzzleOffset)) (Camera|GetCameraRotation (Game|GetPlayerCameraManager 0)) "3.000000,3.000000,3.000000") "Undefined" "MultiplyWithRoot" 0 0))
      (:then_1
        (Class|WeaponBase|ShakeCamera))
      (:then_2
        (Class|WeaponBase|HandleClip))
      (:then_3
        (Audio|PlaySoundatLocation (Variables|Default|GetFiringSound) (Transformation|GetActorLocation) "0, 0, 0" 1.0 1.0 0.0 "/Game/Waves/Sounds/PlayerFireSoundAttenuation.PlayerFireSoundAttenuation" 0 0 0)))))

(fn ConstructionScript)