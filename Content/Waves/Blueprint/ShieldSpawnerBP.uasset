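; ShieldSpawnerBP is an enemy that adds shields, spins and can be destroyed for combo and score.
; BeginPlay adds a shield, and a one-shot timer adds another three seconds later while incrementing NumberOfTentacles; a second timer has no event bound.
; Tick rotates the shielder core and root component at different rates.
; Damage reduces EnemyHealth, and at zero or below the actor destroys itself and applies combo and score.
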(event Custom|CustomEvent
  (Class|ShieldEnemy|AddShield)
  (bind _result (Math|Integer|IncrementInt (Variables|Default|GetNumberOfTentacles))))

(event EventBeginPlay
  (|CallParentFunction)
  (Class|ShieldEnemy|AddShield)
  (Utilities|Time|SetTimerbyEvent (delegate Custom|CustomEvent) 3.0)
  (Utilities|Time|SetTimerbyEvent 0 3.0))

(event EventTick
  (params (DeltaSeconds :type Float%20%28single-precision%29))
  (Transformation|AddWorldRotation (Variables|Default|GetShielderCore) "0.500000,1.000000,0.700000" false false)
  (Transformation|AddWorldRotation (Variables|Default|GetRootEnemyComponent) "0.000000,0.150000,0.000000" false false))

(event EventDamageEnemy
  (params (damageAmount :type Integer))
  (bind _output_get (Variables|Default|SetEnemyHealth (- (Variables|Default|GetEnemyHealth) damageAmount)))
  (if (<= _output_get 0)
    (Actor|DestroyActor)
    (Class|EnemyBase|ApplyComboandScore)))

(fn ConstructionScript)