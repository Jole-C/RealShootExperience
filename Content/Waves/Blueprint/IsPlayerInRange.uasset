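; Behavior tree node for the drone spawner enemy that tracks whether the player is close enough to attack.
; On each AI tick it compares the distance between player pawn 0 and the controlled DroneSpawnerEnemyBP against that enemy's MinimumPlayerDistanceForAttack.
; It writes the result to the IsPlayerInRange blackboard bool through a hard-coded key name, leaving it untouched when the cast fails or the player pawn is invalid.
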(event EventReceiveTickAI
  (params (OwnerController :type AI%20Controller%20Object%20Reference) (ControlledPawn :type Pawn%20Object%20Reference) (DeltaSeconds :type Float%20%28single-precision%29))
  (bind _asdrone_spawner_enemy_bp (Utilities|Casting|CastToDroneSpawnerEnemyBP ControlledPawn))
  (Utilities|IsValid (Game|Player|GetPlayerPawn 0)
    (:Is%20Valid
      (if true
        (Class|BTFunctionLibrary|SetBlackboardValueasBool (Utilities|Struct|MakeBlackboardKeySelector 0 "IsPlayerInRange") (< (Math|Vector|Distance(Vector) (Transformation|GetActorLocation (Game|Player|GetPlayerPawn 0)) (Transformation|GetActorLocation _asdrone_spawner_enemy_bp)) (Variables|/Script/ACTGDFPS502.DroneSpawnerEnemy|GetMinimumPlayerDistanceForAttack _asdrone_spawner_enemy_bp)))))))