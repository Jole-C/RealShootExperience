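; AI controller for the drone spawner enemy, driving its behavior tree and timing its switch into enemy spawning.
; On possess it caches the pawn, then each tick mirrors the pawn's state into the Blackboard.
; Reaching the ATPLAYER state starts the behavior tree once and, if a player pawn exists, a one-shot timer using the pawn's delay.
; When the timer fires, the state becomes ENEMIES and the timer gate resets.
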(event Custom|SpawnEnemies
  ;[1 1 1] If we are spawning enemies, set up the spawning behaviour.
  (Variables|/Script/ACTGDFPS502.DroneSpawnerEnemy|SetEnemyState (Variables|Default|GetAs%20Drone%20Spawner%20Enemy%20BP) "SPAWN_ENEMIES")
  (Utilities|FlowControl|DoOnce false) ; enters at Reset
)

(event EventTick
  (params (DeltaSeconds :type Float%20%28single-precision%29))
  (Utilities|FlowControl|Sequence
    (:then_0
      (Utilities|IsValid (Variables|Default|GetBlackboard)
        (:Is%20Valid
          ;[1 1 1] Update the state in the blackboard
          (AI|Components|Blackboard|SetValueasEnum (Variables|Default|GetBlackboard) (Utilities|Name|MakeLiteralName "SpawnerState") (Variables|/Script/ACTGDFPS502.DroneSpawnerEnemy|GetEnemyState (Variables|Default|GetAs%20Drone%20Spawner%20Enemy%20BP))))))
    (:then_1
      ;[1 1 1] If we are spawning enemies, set up the spawning behaviour.
      (Utilities|IsValid (Game|Player|GetPlayerPawn 0)
        (:Is%20Valid
          (if (Utilities|Enum|Equal(Enum) (Variables|/Script/ACTGDFPS502.DroneSpawnerEnemy|GetEnemyState (Variables|Default|GetAs%20Drone%20Spawner%20Enemy%20BP)) "LOOK_AT_PLAYER")
            (Utilities|FlowControl|DoOnce false
              (:Completed
                (CallFunction|StartonSpawnTimer (delegate Custom|SpawnEnemies))))))))
    (:then_2
      (if (Utilities|Enum|Equal(Enum) (Variables|/Script/ACTGDFPS502.DroneSpawnerEnemy|GetEnemyState (Variables|Default|GetAs%20Drone%20Spawner%20Enemy%20BP)) "LOOK_AT_PLAYER")
        (Utilities|FlowControl|DoOnce false
          (:Completed
            (AI|RunBehaviorTree "/Game/Waves/Blueprint/DroneSpawnerBehaviourTree.DroneSpawnerBehaviourTree")))))))

(event EventPossess
  (params (PossessedPawn :type Pawn%20Object%20Reference))
  ;[1 1 1] On possess, set up reference
  (bind _asdrone_spawner_enemy_bp (Utilities|Casting|CastToDroneSpawnerEnemyBP PossessedPawn))
  (Variables|Default|SetAs%20Drone%20Spawner%20Enemy%20BP _asdrone_spawner_enemy_bp))

(fn ConstructionScript)

(fn StartonSpawnTimer
  (params (Event :type Delegate))
  (bind _returnvalue (Utilities|Time|SetTimerbyEvent Event (Variables|/Script/ACTGDFPS502.DroneSpawnerEnemy|GetTimeUntilSpawnEnemies (Variables|Default|GetAs%20Drone%20Spawner%20Enemy%20BP))))
  (Variables|Default|SetSpawnEnemiesHandle _returnvalue))