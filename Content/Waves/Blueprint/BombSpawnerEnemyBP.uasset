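; BombSpawnerEnemyBP is a wave enemy Blueprint that takes damage and awards combo and score when killed.
; DamageEnemy subtracts damage from EnemyHealth, and at zero or below destroys the actor, then calls ApplyComboAndScore.
; BeginPlay, Tick and EndPlay only forward to the parent class, and no bomb-spawning logic appears in these graphs.
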(event EventBeginPlay
  (|CallParentFunction))

(event EventEndPlay
  (params (EndPlayReason :type EEndPlayReason%20Enum :default "Destroyed"))
  (|CallParentFunction EndPlayReason))

(event EventTick
  (params (DeltaSeconds :type Float%20%28single-precision%29))
  (|CallParentFunction DeltaSeconds))

(event EventDamageEnemy
  (params (damageAmount :type Integer))
  (bind _output_get (Variables|Default|SetEnemyHealth (- (Variables|Default|GetEnemyHealth) damageAmount)))
  (if (<= _output_get 0)
    (Actor|DestroyActor)
    (Class|EnemyBase|ApplyComboandScore)))

(fn ConstructionScript)