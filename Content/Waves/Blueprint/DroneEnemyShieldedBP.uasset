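; Shielded drone enemy that homes in on the player, damaging them and destroying itself when they enter its detection radius.
; Homing uses projectile movement aimed at the character's root, set after a next-frame delay on BeginPlay.
; Tick eases the pitch of meshes tagged "Tooth" between open and closed angles based on IsShieldOpen.
; DamageEnemy subtracts health without checking shield state, destroying the drone and applying combo and score at zero.
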(event Custom|OnComponentBeginOverlap_Event
  (params (OverlappedComponent :type Primitive%20Component%20Object%20Reference) (OtherActor :type Actor%20Object%20Reference) (OtherComp :type Primitive%20Component%20Object%20Reference) (OtherBodyIndex :type Integer) (bFromSweep :type Boolean) (SweepResult :type Hit%20Result%20Structure%20%28by%20ref%29))
  (if (== OtherActor (Game|Player|GetPlayerPawn 0))
    (bind _asbp_first_person_character (Utilities|Casting|CastToBP_FirstPersonCharacter OtherActor))
    (Game|Damage|ApplyDamage _asbp_first_person_character 1.0 0 0)
    (Actor|DestroyActor)))

(event EventBeginPlay
  (|CallParentFunction)
  (Utilities|FlowControl|Sequence
    (:then_0
      (Utilities|FlowControl|Delay 0.0)
      (Variables|/Script/Engine.ProjectileMovementComponent|SetHomingTargetComponent (Variables|Default|GetProjectileMovement) (Variables|/Script/Engine.Actor|GetRootComponent (Variables|Default|GetCharacterReference))))
    (:then_1
      (Collision|AssignOnComponentBeginOverlap (Variables|Default|GetPlayerDetectionRadius) (delegate Custom|OnComponentBeginOverlap_Event)))
    (:then_2
      (Variables|Default|SetTeethComponents (Actor|GetComponentsbyTag "/Script/Engine.StaticMeshComponent" "Tooth")))))

(event Collision|EventActorBeginOverlap
  (params (OtherActor :type Actor%20Object%20Reference)))

(event EventTick
  (params (DeltaSeconds :type Float%20%28single-precision%29))
  (for _array_element (Variables|Default|GetTeethComponents)
    (Transformation|SetRelativeRotation _array_element (Math|Interpolation|RInterpTo (Variables|/Script/Engine.SceneComponent|GetRelativeRotation _array_element) (Math|Rotator|MakeRotator 0.0 (Math|Float|SelectFloat (Variables|Default|GetShieldOpenDegrees) (Variables|Default|GetShieldCloseDegrees) (Variables|Default|GetIsShieldOpen)) 0.0) DeltaSeconds 0.9) false false)))

(event EventDamageEnemy
  (params (damageAmount :type Integer))
  (bind _output_get (Variables|Default|SetEnemyHealth (- (Variables|Default|GetEnemyHealth) damageAmount)))
  (if (<= _output_get 0)
    (Actor|DestroyActor)
    (Class|EnemyBase|ApplyComboandScore)))

(fn ConstructionScript)