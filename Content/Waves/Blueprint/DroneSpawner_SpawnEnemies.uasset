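; A behavior tree task that has a drone spawner enemy spawn a wave of enemies.
; On its first tick it starts a wave on the pawn's EnemySpawner, then keeps turning the pawn toward the player every tick.
; It finishes successfully and resets its do-once gate when spawning stops, or fails with a debug message if the player pawn is invalid.
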(event EventReceiveTickAI
  (params (OwnerController :type AI%20Controller%20Object%20Reference) (ControlledPawn :type Pawn%20Object%20Reference) (DeltaSeconds :type Float%20%28single-precision%29))
  (bind _asdrone_spawner_enemy_bp (Utilities|Casting|CastToDroneSpawnerEnemyBP ControlledPawn))
  (Variables|Default|SetAs%20Drone%20Spawner%20Enemy%20BP _asdrone_spawner_enemy_bp)
  (Utilities|IsValid (Game|Player|GetPlayerPawn 0)
    (:Is%20Valid
      (Utilities|FlowControl|Sequence
        (:then_0
          (Utilities|FlowControl|DoOnce false :!label _label
            (:Completed
              (Class|EnemySpawner|BeginWave (Variables|/Game/Waves/Blueprint/DroneSpawnerEnemyBP.DroneSpawnerEnemyBP_C|GetEnemySpawner (Variables|Default|GetAs%20Drone%20Spawner%20Enemy%20BP))))))
        (:then_1
          (Class|DroneSpawnerEnemy|LookatLocation (Variables|Default|GetAs%20Drone%20Spawner%20Enemy%20BP) (Transformation|GetActorLocation (Game|Player|GetPlayerPawn 0))))
        (:then_2
          (if (not (Variables|/Script/ACTGDFPS502.EnemySpawner|GetIsSpawningEnemies (Variables|/Game/Waves/Blueprint/DroneSpawnerEnemyBP.DroneSpawnerEnemyBP_C|GetEnemySpawner (Variables|Default|GetAs%20Drone%20Spawner%20Enemy%20BP))))
            (AI|BehaviorTree|FinishExecute true)
            (goto _label Reset)))))
    (:Is%20Not%20Valid
      (AI|BehaviorTree|FinishExecute false)
      (Development|PrintString "Drone Spawner - Player is not valid."))))