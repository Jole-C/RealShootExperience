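; Default weapon Blueprint that fires camera-aimed sphere traces at weakpoints and shows its ammo on the HUD.
; BeginPlay adds an ammo widget to the interface controller's canvas, which EndPlay clears.
; When allowed, Fire triggers hit weakpoints with burst effects, resets the score combo on misses or non-weakpoint hits, then plays muzzle effect, camera shake, clip handling and sound.
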(event EventBeginPlay
  (Utilities|FlowControl|Sequence
    (:then_0
      (bind _returnvalue (Actor|GetActorOfClass "/Game/Waves/UI/InterfaceControllerBP.InterfaceControllerBP_C"))
      (bind _output_get (Variables|Default|SetInterfaceControllerReference _returnvalue))
      (bind _returnvalue_2 (UserInterface|CreateWidget "/Game/Waves/UI/WeaponAmmo.WeaponAmmo_C"))
      (bind _output_get_2 (Variables|Default|SetAmmoWidgetReference _returnvalue_2))
      (Class|CanvasPanel|AddChildtoCanvas (Variables|/Game/Waves/UI/Interface.Interface_C|GetWeaponAmmoCanvas (Variables|/Game/Waves/UI/InterfaceControllerBP.InterfaceControllerBP_C|GetWidgetReference _output_get)) _output_get_2)
      (Class|WeaponBase|UpdateHud)
      (Class|UserWidget|SetAnchorsinViewport (Variables|Default|GetAmmoWidgetReference) (Utilities|Struct|MakeAnchors "(X=0.000000,Y=0.000000)" "(X=1.000000,Y=1.000000)")))))

(event EventOnWeaponHitVisuals
  (params (OnWeaponHit :type Vector :default "0, 0, 0"))
  (for _index (range 0 4)
    (Niagara|SpawnSystematLocation "/Game/Waves/Niagara/DefaultWeaponFire.DefaultWeaponFire" OnWeaponHit (Math|Random|RandomRotator false))))

(event EventUpdateHud
  (Utilities|FlowControl|Sequence
    (:then_0
      (Variables|/Script/UMG.TextBlock|SetText (Variables|/Game/Waves/UI/WeaponAmmo.WeaponAmmo_C|GetAmmoClipCurrent (Variables|Default|GetAmmoWidgetReference)) (Utilities|Text|ToText(Integer) (Variables|Default|GetCurrentClip))))
    (:then_1
      (Variables|/Script/UMG.TextBlock|SetText (Variables|/Game/Waves/UI/WeaponAmmo.WeaponAmmo_C|GetAmmoClipMax (Variables|Default|GetAmmoWidgetReference)) (Utilities|Text|ToText(Integer) (Variables|Default|GetMaxClip))))))

(event EventFire
  (bind _returnvalue (Game|GetPlayerCameraManager 0))
  (bind _returnvalue_2 (Camera|GetCameraLocation _returnvalue))
  ;[1 1 1] Generate line trace on hit
  (if (Variables|Default|GetCanFire)
    (Utilities|FlowControl|Sequence
      (:then_0
        (bind (_outhit _returnvalue_3) (Collision|SphereTraceByChannel _returnvalue_2 (+ _returnvalue_2 (* (Transformation|GetWorldRotation (Variables|/Script/Engine.PlayerCameraManager|GetTransformComponent _returnvalue)) (Variables|Default|GetWeaponFireDistance))) 1.3e+02 "TraceTypeQuery3" false 0 "None" true "(R=1.000000,G=0.000000,B=0.000000,A=1.000000)" "(R=0.000000,G=1.000000,B=0.000000,A=1.000000)" 0.0))
        (if _returnvalue_3
          (Utilities|IsValid (.HitComponent (Collision|BreakHitResult _outhit))
            (:Is%20Valid
              (bind _asweakpoint_base (Utilities|Casting|CastToWeakpointBase (Transformation|GetAttachParent (.HitComponent (Collision|BreakHitResult _outhit))))
                (:then
                  (Class|WeakpointBase|OnWeakpointHit _asweakpoint_base)
                  (Class|WeaponBase|OnWeaponHitVisuals (.Location (Collision|BreakHitResult _outhit))))
                (:CastFailed
                  (Development|PrintString "Not a weakpoint")
                  (Class|ScoreManager|ResetCombo (Variables|Default|GetScoreManagerReference)))))
            (:Is%20Not%20Valid
              (Development|PrintString "Object is not valid")))
          (else
            (Class|ScoreManager|ResetCombo (Variables|Default|GetScoreManagerReference)))))
      (:then_1
        (Niagara|SpawnSystematLocation "/Game/Waves/Niagara/DefaultWeaponFire.DefaultWeaponFire" (Transformation|GetWorldLocation (Variables|Default|GetMuzzleOffset)) (Camera|GetCameraRotation (Game|GetPlayerCameraManager 0))))
      (:then_2
        (Class|WeaponBase|ShakeCamera))
      (:then_3
        (Class|WeaponBase|HandleClip))
      (:then_4
        (Audio|PlaySoundatLocation (Variables|Default|GetFiringSound) (Transformation|GetActorLocation) "0, 0, 0" 1.0 1.0 0.0 "/Game/Waves/Sounds/PlayerFireSoundAttenuation.PlayerFireSoundAttenuation" 0 0 0)))))

(event EventEndPlay
  (params (EndPlayReason :type EEndPlayReason%20Enum :default "Destroyed"))
  (Widget|Panel|ClearChildren (Variables|/Game/Waves/UI/Interface.Interface_C|GetWeaponAmmoCanvas (Variables|/Game/Waves/UI/InterfaceControllerBP.InterfaceControllerBP_C|GetWidgetReference (Variables|Default|GetInterfaceControllerReference)))))

(fn ConstructionScript)