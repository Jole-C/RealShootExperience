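; Behavior tree task that keeps a drone spawner enemy facing the player.
; Each AI tick it casts the pawn to DroneSpawnerEnemyBP and passes the first player pawn's location to its LookAtLocation.
; It finishes successfully once the enemy's state is no longer ATPLAYER, or fails with a debug print if the player pawn is invalid.
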(event EventReceiveTickAI
  (params (OwnerController :type AI%20Controller%20Object%20Reference) (ControlledPawn :type Pawn%20Object%20Reference) (DeltaSeconds :type Float%20%28single-precision%29))
  (bind _asdrone_spawner_enemy_bp (Utilities|Casting|CastToDroneSpawnerEnemyBP ControlledPawn))
  (Variables|Default|SetAs%20Drone%20Spawner%20Enemy%20BP _asdrone_spawner_enemy_bp)
  (Utilities|IsValid (Game|Player|GetPlayerPawn 0)
    (:Is%20Valid
      (Utilities|FlowControl|Sequence
        (:then_0
          (Class|DroneSpawnerEnemy|LookatLocation (Variables|Default|GetAs%20Drone%20Spawner%20Enemy%20BP) (Transformation|GetActorLocation (Game|Player|GetPlayerPawn 0))))
        (:then_1
          (if (not (Utilities|Enum|Equal(Enum) (Variables|/Script/ACTGDFPS502.DroneSpawnerEnemy|GetEnemyState (Variables|Default|GetAs%20Drone%20Spawner%20Enemy%20BP)) "LOOK_AT_PLAYER"))
            (AI|BehaviorTree|FinishExecute true)))))
    (:Is%20Not%20Valid
      (AI|BehaviorTree|FinishExecute false)
      (Development|PrintString "Drone Spawner - Player is not valid."))))