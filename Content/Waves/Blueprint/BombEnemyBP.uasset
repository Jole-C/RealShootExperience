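; Bomb enemy that optionally homes in on the player and explodes on a fuse once the player is nearby.
; An overlap on PlayerDetectionRadius starts a one-shot timer to Explode and sets IsSetToExplode.
; Explode damages a player still in range, then destroys the actor.
; It can also trigger overlapping bombs, but only if its own IsSetToExplode is false, so fuse-triggered blasts do not chain.
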(event Custom|OnComponentBeginOverlap_Event
  (params (OverlappedComponent :type Primitive%20Component%20Object%20Reference) (OtherActor :type Actor%20Object%20Reference) (OtherComp :type Primitive%20Component%20Object%20Reference) (OtherBodyIndex :type Integer) (bFromSweep :type Boolean) (SweepResult :type Hit%20Result%20Structure%20%28by%20ref%29))
  ;[1 1 1] Once the player is within the trigger radius, start the fuse for the explosion, and stop the overlap event from firing again
  (if (not (Utilities|Time|IsTimerActivebyHandle (Variables|Default|GetExplosionTimer)))
    (bind _array_element (Utilities|Array|ForEachLoopwithBreak (Collision|GetOverlappingActors (Variables|Default|GetPlayer%20Detection%20Radius) "/Game/FirstPerson/Blueprints/BP_FirstPersonCharacter.BP_FirstPersonCharacter_C" :!class /Script/Engine.PrimitiveComponent) :!label _label)
      (:LoopBody
        (if (== (Utilities|GetClass _array_element) "/Game/FirstPerson/Blueprints/BP_FirstPersonCharacter.BP_FirstPersonCharacter_C")
          (Utilities|FlowControl|Sequence
            (:then_0
              (bind _returnvalue (Utilities|Time|SetTimerbyEvent (delegate EventExplode) (Variables|Default|GetFuseTimeSeconds)))
              (Variables|Default|SetExplosionTimer _returnvalue)
              (Variables|Default|SetIsSetToExplode true))
            (:then_1
              (goto _label Break))))))))

(event EventBeginPlay
  (|CallParentFunction)
  (Utilities|FlowControl|Sequence
    (:then_0
      ;[1 1 1] If this component should home in, set that up
      (Variables|/Script/Engine.ProjectileMovementComponent|SetbIsHomingProjectile (Variables|Default|GetProjectileMovement) (Variables|Default|GetShouldHome))
      (Variables|/Script/Engine.ProjectileMovementComponent|SetHomingTargetComponent (Variables|Default|GetProjectileMovement) (Variables|/Script/Engine.Actor|GetRootComponent (Game|Player|GetPlayerPawn 0))))
    (:then_1
      (Collision|AssignOnComponentBeginOverlap (Variables|Default|GetPlayer%20Detection%20Radius) (delegate Custom|OnComponentBeginOverlap_Event)))))

(event EventEndPlay
  (params (EndPlayReason :type EEndPlayReason%20Enum :default "Destroyed"))
  (|CallParentFunction EndPlayReason))

(event EventExplode
  ;[1 1 1] Explode the enemy, and if the player is still within range, damage them
  (Utilities|FlowControl|Sequence
    (:then_0
      (for _array_element (Collision|GetOverlappingActors (Variables|Default|GetPlayer%20Detection%20Radius) "BombEnemyBP_C" :!class /Script/Engine.PrimitiveComponent)
        (bind _asbomb_enemy_bp (Utilities|Casting|CastToBombEnemyBP _array_element))
        (if (not (Variables|Default|GetIsSetToExplode))
          (Utilities|FlowControl|Sequence
            (:then_0
              (Class|BombEnemy|Explode _asbomb_enemy_bp))
            (:then_1
              (Variables|BombEnemyBP_C|SetIsSetToExplode _asbomb_enemy_bp true))))))
    (:then_1
      (bind _array_element_2 (Utilities|Array|ForEachLoopwithBreak (Collision|GetOverlappingActors (Variables|Default|GetPlayer%20Detection%20Radius) 0 :!class /Script/Engine.PrimitiveComponent) :!label _label)
        (:LoopBody
          (if (== _array_element_2 (Game|Player|GetPlayerPawn 0))
            (Game|Damage|ApplyDamage _array_element_2 1.0 0 0)
            (goto _label Break)))))
    (:then_2
      (Actor|DestroyActor))))

(fn ConstructionScript)