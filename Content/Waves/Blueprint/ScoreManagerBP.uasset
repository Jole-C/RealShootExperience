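; Score manager Blueprint that shows the score and combo on the in-game interface.
; On BeginPlay it finds and caches the InterfaceControllerBP actor.
; SetComboVisuals writes "Score X Combo" to that controller's widget ScoreText, prefixing the score with a single zero and keeping at most its rightmost six characters.
; The graphs only display Score and Combo; neither value is changed here.
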(event EventBeginPlay
  (bind _returnvalue (Actor|GetActorOfClass "/Game/Waves/UI/InterfaceControllerBP.InterfaceControllerBP_C"))
  (Variables|Default|SetInterfaceControllerReference _returnvalue))

(event EventSetComboVisuals
  (Variables|/Script/UMG.TextBlock|SetText (Variables|/Game/Waves/UI/Interface.Interface_C|GetScoreText (Variables|/Game/Waves/UI/InterfaceControllerBP.InterfaceControllerBP_C|GetWidgetReference (Variables|Default|GetInterfaceControllerReference))) (Utilities|Text|FormatText "{Score} X {Combo}" (Utilities|String|Right (Utilities|String|Append "0" (Utilities|String|ToString(Integer) (Variables|Default|GetScore))) 6) (Variables|Default|GetCombo))))

(fn ConstructionScript)