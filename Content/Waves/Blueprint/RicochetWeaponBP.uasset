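; Ricochet weapon Blueprint that damages weakpoints and can bounce a shot to another nearby one.
; Fire sphere-traces from the camera, calls OnWeakpointHit, and resets the score combo on a miss or non-weakpoint hit.
; A weighted roll triggers a multi-sphere trace around the hit, picking a random second weakpoint, with delayed sound and Niagara effects.
; It also handles camera shake and clip, and owns an ammo widget on the HUD canvas.
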(event EventBeginPlay
  (bind _returnvalue (Actor|GetActorOfClass "/Game/Waves/UI/InterfaceControllerBP.InterfaceControllerBP_C"))
  (bind _output_get (Variables|Default|SetInterfaceControllerReference _returnvalue))
  (bind _returnvalue_2 (UserInterface|CreateWidget "/Game/Waves/UI/WeaponAmmo.WeaponAmmo_C"))
  (bind _output_get_2 (Variables|Default|SetAmmoWidgetReference _returnvalue_2))
  (Class|CanvasPanel|AddChildtoCanvas (Variables|/Game/Waves/UI/Interface.Interface_C|GetWeaponAmmoCanvas (Variables|/Game/Waves/UI/InterfaceControllerBP.InterfaceControllerBP_C|GetWidgetReference _output_get)) _output_get_2)
  (Class|UserWidget|SetAnchorsinViewport (Variables|Default|GetAmmoWidgetReference) (Utilities|Struct|MakeAnchors "(X=0.000000,Y=0.000000)" "(X=1.000000,Y=1.000000)")))

(event EventOnWeaponHitVisuals
  (params (OnWeaponHit :type Vector :default "0, 0, 0"))
  (for _index (range 0 4)
    (Niagara|SpawnSystematLocation "/Game/Waves/Niagara/RicochetWeaponFire.RicochetWeaponFire" OnWeaponHit (Math|Random|RandomRotator false))))

(event EventTick
  (params (DeltaSeconds :type Float%20%28single-precision%29)))

(event Collision|EventActorBeginOverlap
  (params (OtherActor :type Actor%20Object%20Reference)))

(event EventUpdateHud
  (Utilities|FlowControl|Sequence
    (:then_0
      (Variables|/Script/UMG.TextBlock|SetText (Variables|/Game/Waves/UI/WeaponAmmo.WeaponAmmo_C|GetAmmoClipCurrent (Variables|Default|GetAmmoWidgetReference)) (Utilities|Text|ToText(Integer) (Variables|Default|GetCurrentClip))))
    (:then_1
      (Variables|/Script/UMG.TextBlock|SetText (Variables|/Game/Waves/UI/WeaponAmmo.WeaponAmmo_C|GetAmmoClipMax (Variables|Default|GetAmmoWidgetReference)) (Utilities|Text|ToText(Integer) (Variables|Default|GetMaxClip))))))

(event EventFire
  (bind _returnvalue (Game|GetPlayerCameraManager 0))
  (bind _returnvalue_2 (Camera|GetCameraLocation _returnvalue))
  ;[1 1 1] Generate line trace on hit
  (if (Variables|Default|GetCanFire)
    (Utilities|FlowControl|Sequence
      (:then_0
        (bind (_outhit _returnvalue_3) (Collision|SphereTraceByChannel _returnvalue_2 (+ _returnvalue_2 (* (Transformation|GetWorldRotation (Variables|/Script/Engine.PlayerCameraManager|GetTransformComponent _returnvalue)) (Variables|Default|GetWeaponFireDistance))) 1.3e+02 "TraceTypeQuery3" false 0 "None" true "(R=1.000000,G=0.000000,B=0.000000,A=1.000000)" "(R=0.000000,G=1.000000,B=0.000000,A=1.000000)" 1e+03))
        (Utilities|FlowControl|Sequence
          (:then_0
            (if _returnvalue_3
              (Utilities|IsValid (.HitComponent (Collision|BreakHitResult _outhit))
                (:Is%20Valid
                  (bind _asweakpoint_base (Utilities|Casting|CastToWeakpointBase (Transformation|GetAttachParent (.HitComponent (Collision|BreakHitResult _outhit))))
                    (:then
                      (Class|WeakpointBase|OnWeakpointHit _asweakpoint_base)
                      ;[1 1 1] Rando mchance to ricochet to another weakpoint
                      (if (Math|Random|RandomBoolwithWeight (Variables|Default|GetPercentageChanceToRicochet))
                        (bind _outhits (Collision|MultiSphereTraceByChannel (Transformation|GetWorldLocation (.HitComponent (Collision|BreakHitResult _outhit))) (Transformation|GetWorldLocation (.HitComponent (Collision|BreakHitResult _outhit))) (Variables|Default|GetRadiusToCheckForOtherWeakpoints) "TraceTypeQuery3" false (Utilities|Array|MakeArray (.HitActor (Collision|BreakHitResult _outhit))) "None"))
                        (if (Utilities|Array|IsNotEmpty _outhits)
                          (Variables|Default|SetRicochetTargets _outhits)
                          (Variables|Default|SetSecondEnemyImpact (.Location (Collision|BreakHitResult (.OutItem (Utilities|Array|Random (Variables|Default|GetRicochetTargets))))))
                          (Utilities|IsValid (.HitComponent (Collision|BreakHitResult (.OutItem (Utilities|Array|Random (Variables|Default|GetRicochetTargets)))))
                            (:Is%20Valid
                              (bind _asweakpoint_base_2 (Utilities|Casting|CastToWeakpointBase (Transformation|GetAttachParent (.HitComponent (Collision|BreakHitResult (.OutItem (Utilities|Array|Random (Variables|Default|GetRicochetTargets))))))))
                              (Utilities|FlowControl|Sequence
                                (:then_0
                                  (Class|WeakpointBase|OnWeakpointHit _asweakpoint_base_2))
                                (:then_1
                                  (Utilities|FlowControl|Delay 0.2)
                                  (Utilities|FlowControl|Sequence
                                    (:then_0
                                      (Audio|PlaySoundatLocation (Variables|Default|GetFiringSound) (Transformation|GetActorLocation) "0, 0, 0" 1.0 1.0 0.0 "/Game/Waves/Sounds/PlayerFireSoundAttenuation.PlayerFireSoundAttenuation" 0 0 0))
                                    (:then_1
                                      (bind _returnvalue_4 (Niagara|SpawnSystematLocation "/Game/Waves/Niagara/RicochetWeaponFire.RicochetWeaponFire" "0, 0, 0" (Math|Rotator|FindLookatRotation (Variables|Default|GetInitialEnemyImpact) (Variables|Default|GetSecondEnemyImpact))))
                                      (Niagara|SetNiagaraVariable(Vector3) _returnvalue_4 "BeamLength" (Math|Vector|GetUnitDirection(Vector) (Variables|Default|GetInitialEnemyImpact) (Variables|Default|GetSecondEnemyImpact))))
                                    (:then_2
                                      (Class|WeaponBase|OnWeaponHitVisuals (Variables|Default|GetSecondEnemyImpact)))))))))))
                    (:CastFailed
                      (Development|PrintString "Not a weakpoint")
                      (Class|ScoreManager|ResetCombo (Variables|Default|GetScoreManagerReference))))))
              (else
                (Class|ScoreManager|ResetCombo (Variables|Default|GetScoreManagerReference)))))
          (:then_1
            (Variables|Default|SetInitialEnemyImpact (.Location (Collision|BreakHitResult _outhit))))))
      (:then_1
        (Class|WeaponBase|ShakeCamera))
      (:then_2
        (Class|WeaponBase|HandleClip))
      (:then_3
        (Audio|PlaySoundatLocation (Variables|Default|GetFiringSound) (Transformation|GetActorLocation) "0, 0, 0" 1.0 1.0 0.0 "/Game/Waves/Sounds/PlayerFireSoundAttenuation.PlayerFireSoundAttenuation" 0 0 0))
      (:then_4
        (Niagara|SpawnSystematLocation "/Game/Waves/Niagara/RicochetWeaponFire.RicochetWeaponFire" (Transformation|GetWorldLocation (Variables|Default|GetMuzzleOffset)) (Camera|GetCameraRotation (Game|GetPlayerCameraManager 0)))))))

(event EventEndPlay
  (params (EndPlayReason :type EEndPlayReason%20Enum :default "Destroyed"))
  (Widget|Panel|ClearChildren (Variables|/Game/Waves/UI/Interface.Interface_C|GetWeaponAmmoCanvas (Variables|/Game/Waves/UI/InterfaceControllerBP.InterfaceControllerBP_C|GetWidgetReference (Variables|Default|GetInterfaceControllerReference)))))

(fn ConstructionScript)