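; Drone spawner enemy with a snake skeleton that spawns default enemies when its EnemySpawner component fires, oriented to the head target root.
; A short timer after BeginPlay switches it to the ATPLAYER state, then self-rescheduling random timers pick head roll targets that Tick interpolates toward.
; Tick pushes state, head targets, roll and spawning flag into the animation blueprints of both main and wireframe meshes.
; Lethal damage destroys it and applies combo and score.
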(event Custom|GenerateRandomRoll
  ;[1 1 1] Generate the random roll for the head
  (Variables|Default|SetTargetHeadRoll (Math|Random|RandomFloatinRange 0.0 3.6e+02))
  (Utilities|Time|SetTimerbyEvent (delegate Custom|GenerateRandomRoll) (Math|Random|RandomFloatinRange 0.25 2.0)))

(event Custom|SetHasPlayedAnimation
  ;[1 1 1] Handle the intro state
  (Variables|Default|SetEnemyState "LOOK_AT_PLAYER")
  (Utilities|Time|SetTimerbyEvent (delegate Custom|GenerateRandomRoll) 1.0))

(event Custom|OnEnemySpawn_Event
  (params (SpawnerLocation :type Vector))
  ;[1 1 1] Spawn enemies
  (Game|SpawnActorfromClass "/Game/Waves/Blueprint/DefaultEnemyBP.DefaultEnemyBP_C" (Math|Transform|MakeTransform SpawnerLocation (Transformation|GetWorldRotation (Variables|Default|GetHeadTargetRoot))) "Undefined" "MultiplyWithRoot" 0 0))

(event EventBeginPlay
  (Utilities|FlowControl|Sequence
    (:then_0
      (EventDispatchers|BindEventtoOnEnemySpawn (Variables|Default|GetEnemySpawner) (delegate Custom|OnEnemySpawn_Event)))
    (:then_1
      ;[1 1 1] Handle the intro state
      (Utilities|Time|SetTimerbyEvent (delegate Custom|SetHasPlayedAnimation) 0.3))
    (:then_2
      (Variables|Default|SetTargetHeadLocation (Transformation|GetWorldLocation (Variables|Default|GetHeadTarget))))))

(event EventDamageEnemy
  (params (damageAmount :type Integer))
  ;[1 1 1] Handle damage
  (bind _output_get (Variables|Default|SetEnemyHealth (- (Variables|Default|GetEnemyHealth) damageAmount)))
  (if (<= _output_get 0)
    (Actor|DestroyActor)
    (Class|EnemyBase|ApplyComboandScore)))

(event EventTick
  (params (DeltaSeconds :type Float%20%28single-precision%29))
  ;[1 1 1] Pass generated variables to the animation blueprint and interpolate the head roll
  (|CallParentFunction DeltaSeconds)
  (Utilities|FlowControl|Sequence
    (:then_0
      ;;[1 1 1] Finalise and setup animation variables
      (Utilities|FlowControl|Sequence
        (:then_0
          (CallFunction|SetAnimationVariables (Variables|Character|GetMesh)))
        (:then_1
          (CallFunction|SetAnimationVariables (Variables|Default|GetWireframeMesh)))))
    (:then_1
      (Variables|Default|SetCurrentHeadRoll (Math|Interpolation|FInterpTo (Variables|Default|GetCurrentHeadRoll) (Variables|Default|GetTargetHeadRoll) DeltaSeconds 3.0)))))

(fn ConstructionScript)

(fn SetAnimationVariables
  (params (Mesh :type Skeletal%20Mesh%20Component%20Object%20Reference))
  (bind _asdronespawner_snake_skeleton_anim_blueprint (Utilities|Casting|CastTodronespawner_snake_Skeleton_AnimBlueprint (Components|SkeletalMesh|GetAnimInstance Mesh))
    (:then
      (LocalVariables|SetAs%20anim%20blueprint _asdronespawner_snake_skeleton_anim_blueprint)
      (Utilities|FlowControl|Sequence
        (:then_0
          (Variables|/Game/Waves/Meshes/DroneSpawner/dronespawner_snake_Skeleton_AnimBlueprint.dronespawner_snake_Skeleton_AnimBlueprint_C|SetAnim_TargetHeadLocation (LocalVariables|GetAs%20anim%20blueprint) (Variables|Default|GetTargetHeadLocation)))
        (:then_1
          (Variables|/Game/Waves/Meshes/DroneSpawner/dronespawner_snake_Skeleton_AnimBlueprint.dronespawner_snake_Skeleton_AnimBlueprint_C|SetEnemySpawningState (LocalVariables|GetAs%20anim%20blueprint) (Variables|Default|GetEnemyState)))
        (:then_2
          (Variables|/Game/Waves/Meshes/DroneSpawner/dronespawner_snake_Skeleton_AnimBlueprint.dronespawner_snake_Skeleton_AnimBlueprint_C|SetAnim_TargetHeadLookLocation (LocalVariables|GetAs%20anim%20blueprint) (Variables|Default|GetTargetHeadLookLocation)))
        (:then_3
          (Variables|/Game/Waves/Meshes/DroneSpawner/dronespawner_snake_Skeleton_AnimBlueprint.dronespawner_snake_Skeleton_AnimBlueprint_C|SetIsSpawningDrones (LocalVariables|GetAs%20anim%20blueprint) (Variables|/Script/ACTGDFPS502.EnemySpawner|GetIsSpawningEnemies (Variables|Default|GetEnemySpawner))))
        (:then_4
          (Variables|/Game/Waves/Meshes/DroneSpawner/dronespawner_snake_Skeleton_AnimBlueprint.dronespawner_snake_Skeleton_AnimBlueprint_C|SetAnim_HeadRoll (LocalVariables|GetAs%20anim%20blueprint) (Variables|Default|GetCurrentHeadRoll)))
        (:then_5
          (return))))
    (:CastFailed
      (Development|PrintString "Could not cast.")
      (return))))

(fn CalculateRelativeSpaceOfVector
  (params (InputVector :type Vector))
  (return (- InputVector (Transformation|GetActorLocation))))