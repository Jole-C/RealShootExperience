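; Bonus enemy actor that drifts through random orientations and triggers a weapon pickup reward when killed.
; A looping timer picks a new random target rotation, and Tick eases toward it with a small quaternion slerp each frame.
; DamageEnemy subtracts health and, at zero or below, destroys the actor and spawns a WeaponPickupHudHandlerBP at the world origin.
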(event Custom|GenerateRotator
  (Variables|Default|SetTargetRotator (Math|Random|RandomRotator false)))

(event EventBeginPlay
  (Utilities|Time|SetTimerbyEvent (delegate Custom|GenerateRotator) (Variables|Default|GetRotationTime) true))

(event EventEndPlay
  (params (EndPlayReason :type EEndPlayReason%20Enum :default "Destroyed"))
  (|CallParentFunction EndPlayReason))

(event EventTick
  (params (DeltaSeconds :type Float%20%28single-precision%29))
  (Transformation|SetActorRotation (Class|KismetMathLibrary|QuatRotator (Class|KismetMathLibrary|QuatSlerp (Math|Conversions|ToQuaternion(Rotator) (Transformation|GetActorRotation)) (Math|Conversions|ToQuaternion(Rotator) (Variables|Default|GetTargetRotator)) 0.01))))

(event EventDamageEnemy
  (params (damageAmount :type Integer))
  (bind _output_get (Variables|Default|SetEnemyHealth (- (Variables|Default|GetEnemyHealth) damageAmount)))
  (if (<= _output_get 0)
    (Actor|DestroyActor)
    (Game|SpawnActorfromClass "/Game/Waves/UI/WeaponPickupHudHandlerBP.WeaponPickupHudHandlerBP_C" (Math|Transform|MakeTransform "0, 0, 0") "Undefined" "MultiplyWithRoot" 0 0)))

(fn ConstructionScript)